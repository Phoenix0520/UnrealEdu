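; BP_03_02_Trace is an actor that chases a referenced Other actor and quits the game when it gets within range.
; Each Tick, while farther than Distance, it steps along the normalized direction to Other, scaled by Speed and delta time for frame-rate independent movement.
; The move sets the actor location directly without sweep, so it ignores blocking collision along the way.
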(event `self.ReceiveTick`
  (params (DeltaSeconds :type "Float (single-precision)"))
  (bind _returnvalue (`self.K2_GetActorLocation`))
  (if (> (`self.GetDistanceTo` (`self.Other`)) (`self.Distance`))
    (`self.K2_SetActorLocation` (+ (* (`KismetMathLibrary.Normal` (- (`self.K2_GetActorLocation` (`self.Other`)) _returnvalue)) (* DeltaSeconds (`self.Speed`))) _returnvalue))
    (else
      (`KismetSystemLibrary.QuitGame` null "Quit"))))

(fn `UserConstructionScript`)